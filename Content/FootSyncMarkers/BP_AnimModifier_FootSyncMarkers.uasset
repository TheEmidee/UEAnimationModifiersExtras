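; Animation modifier that auto-generates foot sync markers on animation sequences whose path passes a name filter.
; Per frame, it dots each configured bone's 2D offset from a reference bone with a direction, adding a marker when the sign flips negative.
; That direction comes from an override or the best token match in the asset path.
; Optional debug curves record the dot; revert can delete the track and curves.
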(event EventOnApply
  (params (AnimationSequence :type Anim%20Sequence%20Object%20Reference))
  ;[1 1 1] Apply
  (if (CallFunction|CanApplyAnimationModifier AnimationSequence)
    (if (not (CallFunction|DoesAnimNotifyTrackExist AnimationSequence))
      (Utilities|FlowControl|Sequence
        (:then_0
          (CallFunction|CreateSyncMarkersforAllBones AnimationSequence (CallFunction|GetReferenceDirection AnimationSequence)))
        (:then_1
          (Class|AnimationBlueprintLibrary|FinalizeBoneAnimation AnimationSequence))))
    (else
      (CallFunction|Log "The animation name did not pass the filter" AnimationSequence))))

(event EventOnRevert
  (params (AnimationSequence :type Anim%20Sequence%20Object%20Reference))
  ;[1 1 1] Revert. Delete all curves and tracks
  (if (CallFunction|CanApplyAnimationModifier AnimationSequence)
    (if (Variables|Setup|GetDeleteExisitingFootSyncTracksOnRevert)
      (Class|AnimationBlueprintLibrary|RemoveAnimationNotifyTrack AnimationSequence (Variables|Setup|SyncMarkers|GetSyncMarkerName))
      (for _array_element (Variables|Setup|Bones|GetBoneSetup)
        (Class|AnimationBlueprintLibrary|RemoveCurve AnimationSequence (.bonename _array_element) false)))))

(fn CanApplyAnimationModifier
  (params (AnimationSequence :type Anim%20Sequence%20Object%20Reference))
  (LocalVariables|SetResult true)
  (LocalVariables|SetAnimationSequencePathName (Class|KismetSystemLibrary|GetPathName AnimationSequence))
  (if (Variables|Setup|GetExecuteEvenIfNameDoesNotMatch)
    (return true)
    (else
      (bind _array_element (Utilities|Array|ForEachLoopwithBreak (Variables|Setup|GetPathFilterNames) :!label _label)
        (:LoopBody
          (bind _output_get (LocalVariables|SetResult (Utilities|String|Contains (LocalVariables|GetAnimationSequencePathName) _array_element)))
          (if _output_get
            (goto _label Break)))
        (:Completed
          (return (LocalVariables|GetResult)))))))

(fn CreateSyncMarkersforAllBones
  (params (AnimationSequence :type Anim%20Sequence%20Object%20Reference) (ReferenceDirection :type Vector%202D%20Structure))
  (Utilities|FlowControl|Sequence
    (:then_0
      (Class|AnimationBlueprintLibrary|AddAnimationNotifyTrack AnimationSequence (Variables|Setup|SyncMarkers|GetSyncMarkerName) "(R=1.000000,G=0.183437,B=0.500461,A=1.000000)")
      (if (Variables|Setup|SyncMarkers|GetAddDebugCurves)
        (for _array_element (Variables|Setup|Bones|GetBoneSetup)
          (Class|AnimationBlueprintLibrary|AddCurve AnimationSequence (.BoneName (Utilities|Struct|BreakBPS_AnimModifier_BoneInfos _array_element)) "RCT_Float" false))))
    (:then_1
      (for _array_element_2 (Variables|Setup|Bones|GetBoneSetup)
        (CallFunction|CreateSyncMarkersforBone AnimationSequence _array_element_2 ReferenceDirection)))))

(fn DoesAnimNotifyTrackExist
  (params (AnimationSequence :type Anim%20Sequence%20Object%20Reference))
  (return (Class|AnimationBlueprintLibrary|IsValidAnimNotifyTrackName AnimationSequence (Variables|Setup|SyncMarkers|GetSyncMarkerName))))

(fn GetReferenceDirection
  (params (AnimationSequence :type Anim%20Sequence%20Object%20Reference))
  (return (select (Math|Vector|Equal(Vector) :A (Variables|Setup|GetReferenceDirectionOverride)) (CallFunction|GetReferenceDirectionfromAssetName AnimationSequence) (Variables|Setup|GetReferenceDirectionOverride))))

(fn Log
  (params (Message :type String) (AnimationSequence :type Anim%20Sequence%20Object%20Reference))
  (Development|PrintString 0 (Utilities|String|Append Message (Class|KismetSystemLibrary|GetPathName AnimationSequence)) false))

(fn CreateSyncMarkersforBone
  (params (AnimationSequence :type Anim%20Sequence%20Object%20Reference) (BoneData :type BPS%20Anim%20Modifier%20Bone%20Infos%20Structure) (ReferenceDirection :type Vector%202D%20Structure))
  (bind (_bonename _syncmarkername) (Utilities|Struct|BreakBPS_AnimModifier_BoneInfos BoneData))
  (LocalVariables|SetLocalReferenceDirection ReferenceDirection)
  (LocalVariables|SetAnimSequence AnimationSequence)
  (LocalVariables|SetFootMarkerName _syncmarkername)
  (LocalVariables|SetCurrentFootBoneName _bonename)
  ;[1 1 1] For each frame of the animation:
  (for _index (range 0 (Class|AnimationBlueprintLibrary|GetNumFrames AnimationSequence))
    ;;[1 1 1] 1. Compute the dot product between the pelvis position and the bone position
    (LocalVariables|SetCurrentTime (CallFunction|GetTimefromFrame (LocalVariables|GetAnimSequence) _index))
    (LocalVariables|SetCurrentDot (Math|Vector2D|DotProduct(2D) (Math|Conversions|ToVector2D(Vector) (- (CallFunction|GetBoneLocationRelativetoatTime (LocalVariables|GetCurrentFootBoneName) (LocalVariables|GetCurrentTime) (LocalVariables|GetAnimSequence)) (CallFunction|GetBoneLocationRelativetoatTime (Variables|Setup|Bones|GetReferenceBoneName) (LocalVariables|GetCurrentTime) (LocalVariables|GetAnimSequence)))) (LocalVariables|GetLocalReferenceDirection)))
    ;;[1 1 1] If the dot product sign changes and if < 0, this means the bone crossed the axis from the pelvis to the ground
    (LocalVariables|SetCurrentDotSign (Math|Float|Sign(Float) (Math|Vector2D|DotProduct(2D) (Math|Conversions|ToVector2D(Vector) (- (CallFunction|GetBoneLocationRelativetoatTime (LocalVariables|GetCurrentFootBoneName) (LocalVariables|GetCurrentTime) (LocalVariables|GetAnimSequence)) (CallFunction|GetBoneLocationRelativetoatTime (Variables|Setup|Bones|GetReferenceBoneName) (LocalVariables|GetCurrentTime) (LocalVariables|GetAnimSequence)))) (LocalVariables|GetLocalReferenceDirection))))
    (if (Math|Boolean|ANDBoolean (> _index 0) (< (Math|Float|Sign(Float) (Math|Vector2D|DotProduct(2D) (Math|Conversions|ToVector2D(Vector) (- (CallFunction|GetBoneLocationRelativetoatTime (LocalVariables|GetCurrentFootBoneName) (LocalVariables|GetCurrentTime) (LocalVariables|GetAnimSequence)) (CallFunction|GetBoneLocationRelativetoatTime (Variables|Setup|Bones|GetReferenceBoneName) (LocalVariables|GetCurrentTime) (LocalVariables|GetAnimSequence)))) (LocalVariables|GetLocalReferenceDirection))) 0.0) (!= (Math|Float|Sign(Float) (Math|Vector2D|DotProduct(2D) (Math|Conversions|ToVector2D(Vector) (- (CallFunction|GetBoneLocationRelativetoatTime (LocalVariables|GetCurrentFootBoneName) (LocalVariables|GetCurrentTime) (LocalVariables|GetAnimSequence)) (CallFunction|GetBoneLocationRelativetoatTime (Variables|Setup|Bones|GetReferenceBoneName) (LocalVariables|GetCurrentTime) (LocalVariables|GetAnimSequence)))) (LocalVariables|GetLocalReferenceDirection))) (LocalVariables|GetLastDotSign)))
      ;;[1 1 1] Then add a marker on the track
      (Class|AnimationBlueprintLibrary|AddAnimationSyncMarker (LocalVariables|GetAnimSequence) (LocalVariables|GetFootMarkerName) (LocalVariables|GetCurrentTime) (Variables|Setup|SyncMarkers|GetSyncMarkerName)))
    (LocalVariables|SetLastDotSign (LocalVariables|GetCurrentDotSign))
    ;;[1 1 1] Add an entry to the debug curve
    (if (Variables|Setup|SyncMarkers|GetAddDebugCurves)
      (Class|AnimationBlueprintLibrary|AddFloatCurveKey (LocalVariables|GetAnimSequence) (LocalVariables|GetCurrentFootBoneName) (LocalVariables|GetCurrentTime) (LocalVariables|GetCurrentDot)))))

(fn GetReferenceDirectionfromAssetName
  (params (AnimationSequence :type Anim%20Sequence%20Object%20Reference))
  ;[1 1 1] That functions parses the animation name to try to find tokens (Like Forward / Bkwd / 45 / 135 / etc...) and looks for the most appropriate reference direction in the property DotProductReferenceDirections
  (bind _output_get (LocalVariables|SetLocalAnimationSequence AnimationSequence))
  (LocalVariables|SetPathName (Class|KismetSystemLibrary|GetPathName _output_get))
  (for _array_element (Variables|Setup|GetDotProductReferenceDirections)
    (if (> (Utilities|Array|Length (.Names (Utilities|Struct|BreakBPS_AnimModifier_DotReferenceDirection _array_element))) (LocalVariables|GetMaxMatchCount))
      (LocalVariables|SetTempTokensConcat "")
      (LocalVariables|SetMatchCount 0)
      (bind _array_element_2 (Utilities|Array|ForEachLoopwithBreak (.Names (Utilities|Struct|BreakBPS_AnimModifier_DotReferenceDirection _array_element)))
        (:LoopBody
          (LocalVariables|SetTempTokensConcat (Utilities|String|Append (LocalVariables|GetTempTokensConcat) " - " _array_element_2))
          (if (Utilities|String|Contains (LocalVariables|GetPathName) _array_element_2)
            (Math|Integer|IncrementInt (LocalVariables|GetMatchCount))))
        (:Completed
          (if (== (LocalVariables|GetMatchCount) (Utilities|Array|Length (.Names (Utilities|Struct|BreakBPS_AnimModifier_DotReferenceDirection _array_element))))
            (LocalVariables|SetResult true)
            (LocalVariables|SetMaxMatchCount (Utilities|Array|Length (.Names (Utilities|Struct|BreakBPS_AnimModifier_DotReferenceDirection _array_element))))
            (LocalVariables|SetReferenceDirection (.ReferenceDirection (Utilities|Struct|BreakBPS_AnimModifier_DotReferenceDirection _array_element)))
            (LocalVariables|SetMatchingTokens (LocalVariables|GetTempTokensConcat)))))))
  (if (LocalVariables|GetResult)
    (CallFunction|Log (Utilities|String|MakeLiteralString (Utilities|String|Append "Matching tokens : " (LocalVariables|GetMatchingTokens) " - Selected direction : " (Utilities|String|ToString(Vector2d) (LocalVariables|GetReferenceDirection)))) (LocalVariables|GetLocalAnimationSequence))
    (else
      (LocalVariables|SetReferenceDirection "(X=0.000000,Y=1.000000)")
      (CallFunction|Log "Impossible to find a reference direction from the name. Uses default (X:0;Y:1)" (LocalVariables|GetLocalAnimationSequence))))
  (return (LocalVariables|GetReferenceDirection)))

(fn GetTimefromFrame
  (params (AnimationSequence :type Anim%20Sequence%20Object%20Reference) (FrameIndex :type Integer))
  (bind _time (Class|AnimationBlueprintLibrary|GetTimeatFrame AnimationSequence FrameIndex))
  (return (select (== 0 (Class|AnimationBlueprintLibrary|GetNumFrames AnimationSequence)) (- _time 0.001) _time)))

(fn GetBoneLocationRelativetoatTime
  (params (TargetBoneName :type Name) (Time :type Float%20%28single-precision%29) (AnimationSequence :type Anim%20Sequence%20Object%20Reference))
  (LocalVariables|SetTransform (Math|Transform|MakeTransform "0, 0, 0"))
  (bind _array_element (Utilities|Array|ForEachLoopwithBreak (Class|AnimationBlueprintLibrary|FindBonePathtoRoot AnimationSequence TargetBoneName))
    (:LoopBody
      (LocalVariables|SetTransform (Math|Transform|ComposeTransforms (LocalVariables|GetTransform) (Class|AnimationBlueprintLibrary|GetBonePoseforTime AnimationSequence _array_element Time false))))
    (:Completed
      (return (.Location (Math|Transform|BreakTransform (LocalVariables|GetTransform)))))))